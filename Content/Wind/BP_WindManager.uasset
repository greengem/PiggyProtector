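; Wind manager that periodically switches which wind source in the level is active.
; A looping timer started at BeginPlay deactivates every entry in WindSources, then activates one picked at random from a fixed index range.
; A recursive retry aims to avoid repeating the last index, but the random roll is evaluated separately for the check, the stored index and the activation, so repeats remain possible.
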(event `self.ReceiveBeginPlay`
  (`KismetSystemLibrary.K2_SetTimerDelegate` (delegate `ActivateRandomWindSource`) 7.0 true))

(event `ActivateRandomWindSource`
  (for _array_element (`self.WindSources`)
    (`/Game/Wind/BP_WindSource.CustomDeactivate` _array_element))
  (`self.SelectAndActivateRandomWindSource`))

(event `SelectAndActivateRandomWindSource`
  (bind _returnvalue (`KismetMathLibrary.RandomIntegerInRange` 0 7))
  (if (!= _returnvalue (`self.LastActivatedIndex`))
    (set `self.LastActivatedIndex` _returnvalue)
    (`/Game/Wind/BP_WindSource.CustomActivate` (`|GetArrayItem` (`self.WindSources`) _returnvalue))
    (else
      (`self.SelectAndActivateRandomWindSource`))))

(fn `UserConstructionScript`)